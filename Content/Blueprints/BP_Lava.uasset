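; BP_Lava is a lava hazard that delegates its damage to a separate BP_DOTRadius actor.
; Shortly after BeginPlay it spawns that actor at its own transform with a fixed radius and the default DamageAmount.
; When an actor with a HealthComponent starts overlapping the mesh, the spawned actor's damage becomes half that actor's health at that moment.
; When such an actor stops overlapping, the damage resets to the default.
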(event `self.ReceiveBeginPlay`
  (`KismetSystemLibrary.Delay` 0.5)
  (bind _returnvalue (`|SpawnActorFromClass` "/Game/Blueprints/BP_DOTRadius.BP_DOTRadius_C" (`self.GetTransform`) "Undefined" "OverrideRootScale" null (`self.Damage Amount`) 1.0 15.0 150.0 null))
  (set `self.DOT Radius` _returnvalue))

(event `self.StaticMesh.OnComponentBeginOverlap`
  (params (OverlappedComponent :type "PrimitiveComponent Object Reference") (OtherActor :type "Actor Object Reference") (OtherComp :type "PrimitiveComponent Object Reference") (OtherBodyIndex :type Integer) (bFromSweep :type Boolean) (SweepResult :type "HitResult Structure (by ref)"))
  (bind _returnvalue (`self.GetComponentByClass` OtherActor "/Script/Spring2022_Capstone.HealthComponent"))
  (`/Engine/EditorBlueprintResources/StandardMacros.IsValid` _returnvalue
    (:`Is Valid`
      (bind _returnvalue_2 (`HealthComponent.GetHealth` _returnvalue))
      (set `DOTRadius.DamageAmount` (/ _returnvalue_2 2.0) (`self.DOT Radius`)))))

(event `self.StaticMesh.OnComponentEndOverlap`
  (params (OverlappedComponent :type "PrimitiveComponent Object Reference") (OtherActor :type "Actor Object Reference") (OtherComp :type "PrimitiveComponent Object Reference") (OtherBodyIndex :type Integer))
  (`/Engine/EditorBlueprintResources/StandardMacros.IsValid` (`self.GetComponentByClass` OtherActor "/Script/Spring2022_Capstone.HealthComponent")
    (:`Is Valid`
      (set `DOTRadius.DamageAmount` (`self.Damage Amount`) (`self.DOT Radius`)))))

(fn `UserConstructionScript`)