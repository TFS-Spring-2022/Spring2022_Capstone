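; BP_DevShotgun is a shotgun weapon Blueprint that handles overheat effects and floating damage numbers.
; TriggerEffect toggles steam and sparks from the overheat state, while Tick re-targets the sparks from a random crystal socket to a random mesh socket or bone.
; DisplayFloatingDamageNumbers spawns one Niagara system per digit, rotated by controller yaw with random roll, offset sideways, textured per digit, and given a different material on crits.
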(event `self.DisplayFloatingDamageNumbers`
  (params (Location :type "Vector Structure") (DamageAmount :type Integer) (bIsCrit :type Boolean))
  (bind (_returnvalue_roll _returnvalue_pitch _returnvalue_yaw) (`KismetMathLibrary.BreakRotator` (`Controller.GetControlRotation` (`GameplayStatics.GetPlayerController` 0))))
  (for _array_element (`KismetStringLibrary.GetCharacterArrayFromString` (`KismetStringLibrary.Conv_IntToString` DamageAmount))
    (bind _returnvalue (`NiagaraFunctionLibrary.SpawnSystemAtLocation` "/Game/Assets/ParticleEffects/FloatingDamageNumbers/NS_FloatingDamageText.NS_FloatingDamageText" Location (`KismetMathLibrary.MakeRotator` (`KismetMathLibrary.RandomFloatInRange` -15.0 35.0) 180.0 _returnvalue_yaw) (0.3 0.3 0.3)))
    (bind _output_get (set `self.DigitSystem` _returnvalue))
    (if bIsCrit
      (`NiagaraComponent.SetVariableMaterial` (`self.DigitSystem`) "DamageTextMaterial" "/Game/Assets/ParticleEffects/FloatingDamageNumbers/DamageNumberMaterials/M_FloatingDamageNumbers_Vulnerable.M_FloatingDamageNumbers_Vulnerable"))
    (`SceneComponent.K2_AddLocalOffset` _output_get (`KismetMathLibrary.MakeVector` 0.0 (`self.TextOffset`)) false false)
    ;[1 1 1] Numbers must be offset because the number is displayed through an array of FStrings each with its own sprite
    (set `self.TextOffset` (+ (`self.TextOffset`) 12.0))
    (switch `string` _array_element
      (:`0`
        (`NiagaraFunctionLibrary.SetTextureObject` (`self.DigitSystem`) "DamageDigit" "/Game/Assets/ParticleEffects/FloatingDamageNumbers/DamageNumberSprites/T_SkyPiratesFont_0.T_SkyPiratesFont_0"))
      (:`1`
        (`NiagaraFunctionLibrary.SetTextureObject` (`self.DigitSystem`) "DamageDigit" "/Game/Assets/ParticleEffects/FloatingDamageNumbers/DamageNumberSprites/T_SkyPiratesFont_1.T_SkyPiratesFont_1"))
      (:`2`
        (`NiagaraFunctionLibrary.SetTextureObject` (`self.DigitSystem`) "DamageDigit" "/Game/Assets/ParticleEffects/FloatingDamageNumbers/DamageNumberSprites/T_SkyPiratesFont_2.T_SkyPiratesFont_2"))
      (:`3`
        (`NiagaraFunctionLibrary.SetTextureObject` (`self.DigitSystem`) "DamageDigit" "/Game/Assets/ParticleEffects/FloatingDamageNumbers/DamageNumberSprites/T_SkyPiratesFont_3.T_SkyPiratesFont_3"))
      (:`4`
        (`NiagaraFunctionLibrary.SetTextureObject` (`self.DigitSystem`) "DamageDigit" "/Game/Assets/ParticleEffects/FloatingDamageNumbers/DamageNumberSprites/T_SkyPiratesFont_4.T_SkyPiratesFont_4"))
      (:`5`
        (`NiagaraFunctionLibrary.SetTextureObject` (`self.DigitSystem`) "DamageDigit" "/Game/Assets/ParticleEffects/FloatingDamageNumbers/DamageNumberSprites/T_SkyPiratesFont_5.T_SkyPiratesFont_5"))
      (:`6`
        (`NiagaraFunctionLibrary.SetTextureObject` (`self.DigitSystem`) "DamageDigit" "/Game/Assets/ParticleEffects/FloatingDamageNumbers/DamageNumberSprites/T_SkyPiratesFont_6.T_SkyPiratesFont_6"))
      (:`7`
        (`NiagaraFunctionLibrary.SetTextureObject` (`self.DigitSystem`) "DamageDigit" "/Game/Assets/ParticleEffects/FloatingDamageNumbers/DamageNumberSprites/T_SkyPiratesFont_7.T_SkyPiratesFont_7"))
      (:`8`
        (`NiagaraFunctionLibrary.SetTextureObject` (`self.DigitSystem`) "DamageDigit" "/Game/Assets/ParticleEffects/FloatingDamageNumbers/DamageNumberSprites/T_SkyPiratesFont_8.T_SkyPiratesFont_8"))
      (:`9`
        (`NiagaraFunctionLibrary.SetTextureObject` (`self.DigitSystem`) "DamageDigit" "/Game/Assets/ParticleEffects/FloatingDamageNumbers/DamageNumberSprites/T_SkyPiratesFont_9.T_SkyPiratesFont_9"))))
  ;[1 1 1] Reset the offset after all numbers have been displayed
  (set `self.TextOffset` 0.0))

(event `self.ReceiveBeginPlay`
  (set `self.Bones` (`SceneComponent.GetAllSocketNames` (`self.SkeletalMesh`))))

(event `self.ReceiveTick`
  (params (DeltaSeconds :type "Float (single-precision)"))
  (bind _overheatsparks (`self.OverHeatSparks`))
  (`FXSystemComponent.SetVectorParameter` _overheatsparks "Begin_Point" (`KismetArrayLibrary.Array_Random` (`|MakeArray` (`SceneComponent.GetSocketLocation` (`self.SkeletalMesh`) "CrystalSocket1") (`SceneComponent.GetSocketLocation` (`self.SkeletalMesh`) "CrystalSocket2") (`SceneComponent.GetSocketLocation` (`self.SkeletalMesh`) "CrystalSocket3"))))
  (`FXSystemComponent.SetVectorParameter` _overheatsparks "End_Point" (`SceneComponent.GetSocketLocation` (`self.SkeletalMesh`) (`KismetArrayLibrary.Array_Random` (`self.Bones`)))))

(event `self.TriggerEffect`
  (bind _returnvalue (`self.GetIsOverheating`))
  (`ActorComponent.SetActive` (`self.OverheatSteam`) _returnvalue true)
  (`ActorComponent.SetActive` (`self.OverHeatSparks`) _returnvalue true))

(fn `UserConstructionScript`)