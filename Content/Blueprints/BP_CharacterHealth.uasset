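; BP_CharacterHealth is a Blueprint that tracks a PlayerHealth value through damage and healing.
; The AnyDamage event subtracts the damage, then prints "Has died" if health is below zero, or the remaining health otherwise.
; The Heal function adds an unclamped amount and prints a "healed for" message that shows the new total rather than the amount healed.
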(event `self.ReceiveAnyDamage`
  (params (Damage :type "Float (single-precision)") (DamageType :type "DamageType Object Reference") (InstigatedBy :type "Controller Object Reference") (DamageCauser :type "Actor Object Reference"))
  ;[1 1 1] Take Damage
  (set `self.PlayerHealth` (- (`self.PlayerHealth`) Damage))
  (if (< (`self.PlayerHealth`) 0.0)
    (`KismetSystemLibrary.PrintString` "Has died")
    (else
      (`KismetSystemLibrary.PrintString` (`KismetStringLibrary.Conv_DoubleToString` (`self.PlayerHealth`))))))

(fn `Heal`
  (params (HealAmount :type "Float (double-precision)"))
  (bind _output_get (set `self.PlayerHealth` (+ (`self.PlayerHealth`) HealAmount)))
  (`KismetSystemLibrary.PrintString` (`KismetStringLibrary.BuildString_Double` "" "Player healed for : \"" _output_get "\"")))

(fn `UserConstructionScript`)