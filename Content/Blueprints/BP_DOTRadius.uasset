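; BP_DOTRadius is a timed damage-over-time area that destroys itself after CloudSeconds.
; Sphere overlap with an actor that has a HealthComponent stores it as the single target and starts a looping one-second DealDamage timer.
; The first successful tick hits harder than later ones, via a Count that never resets.
; Leaving the sphere clears the target, but the timer keeps running.
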(event `self.ReceiveBeginPlay`
  (`self.SetLifeSpan` (`self.CloudSeconds`)))

(event `self.SphereCollision.OnComponentBeginOverlap`
  (params (OverlappedComponent :type "PrimitiveComponent Object Reference") (OtherActor :type "Actor Object Reference") (OtherComp :type "PrimitiveComponent Object Reference") (OtherBodyIndex :type Integer) (bFromSweep :type Boolean) (SweepResult :type "HitResult Structure (by ref)"))
  (`/Engine/EditorBlueprintResources/StandardMacros.IsValid` (`self.GetComponentByClass` OtherActor "/Script/Spring2022_Capstone.HealthComponent")
    (:`Is Valid`
      (set `self.OtherCharRef` OtherActor)
      (`KismetSystemLibrary.K2_SetTimer` null "DealDamage" 1.0 true))))

(event `DealDamage`
  (if (== (`self.Count`) 0)
    (bind _othercharref (`self.OtherCharRef`)
      (:`then`
        (`GameplayStatics.ApplyDamage` _othercharref 10.0))
      (:`else`))
    (else
      (bind _othercharref_2 (`self.OtherCharRef`)
        (:`then`
          (`GameplayStatics.ApplyDamage` _othercharref_2 5.0))
        (:`else`))))
  (`/Engine/EditorBlueprintResources/StandardMacros.IncrementInt` (`self.Count`)
    (:`  `
      (`KismetSystemLibrary.PrintString` "Dealing X Damage to player"))))

(event `self.SphereCollision.OnComponentEndOverlap`
  (params (OverlappedComponent :type "PrimitiveComponent Object Reference") (OtherActor :type "Actor Object Reference") (OtherComp :type "PrimitiveComponent Object Reference") (OtherBodyIndex :type Integer))
  (if (== OtherActor (`self.OtherCharRef`))
    (set `self.OtherCharRef` null)))

(fn `UserConstructionScript`)