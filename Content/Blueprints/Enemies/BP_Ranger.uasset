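; BP_Ranger is an enemy character Blueprint that handles hit reactions, navigation jumps and combat range.
; Hit reactions map the struck bone to a section of the grunt hit montage by body region, with random picks for the right arm and unmatched bones.
; Jumps launch the character along a suggested projectile arc aimed above the destination, with jump and landing montages.
; GetIdealRange returns fixed attack and defend radii.
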(event `self.PlayHitAnimation`
  (params (HitBone :type Name))
  ;[1 1 1] Play Hit Animation
  (switch `name` HitBone
    (:`Default`
      (if (`KismetMathLibrary.RandomBool`)
        (`self.PlayAnimMontage` "/Game/Blueprints/Enemies/AM_GruntHit.AM_GruntHit" 1.0 "NoROOT_RightShoulderHit1")
        (else
          (`self.PlayAnimMontage` "/Game/Blueprints/Enemies/AM_GruntHit.AM_GruntHit" 1.0 "NoROOT_RightShoulderHit2"))))
    (:`Grunt_Head`
      (`self.PlayAnimMontage` "/Game/Blueprints/Enemies/AM_GruntHit.AM_GruntHit" 1.0 "ROOT_LeftHeadKnockBackHit" :!label _label))
    (:`Grunt_Neck2`
      (goto _label))
    (:`Grunt_Neck1`
      (goto _label))
    (:`Grunt_RightShoulder`
      (switch `int` (`KismetMathLibrary.RandomIntegerInRange` 0 2) :!label _label_2
        (:`Default`
          (`self.PlayAnimMontage` "/Game/Blueprints/Enemies/AM_GruntHit.AM_GruntHit" 1.0 "ROOT_RightShoulderHit2" :!label _label_3))
        (:`0`
          (goto _label_3))
        (:`1`
          (`self.PlayAnimMontage` "/Game/Blueprints/Enemies/AM_GruntHit.AM_GruntHit" 1.0 "NoROOT_RightShoulderHit1"))
        (:`2`
          (`self.PlayAnimMontage` "/Game/Blueprints/Enemies/AM_GruntHit.AM_GruntHit" 1.0 "NoROOT_RightShoulderHit2"))))
    (:`Grunt_RightArm`
      (goto _label_2))
    (:`Grunt_RightForeArm`
      (goto _label_2))
    (:`Grunt_LeftShoulder`
      (`self.PlayAnimMontage` "/Game/Blueprints/Enemies/AM_GruntHit.AM_GruntHit" 1.0 "ROOT_LeftShoulderKnockBack" :!label _label_4))
    (:`Grunt_LeftArm`
      (goto _label_4))
    (:`Grunt_LeftForeArm`
      (goto _label_4))
    (:`Grunt_Hips`
      (`self.PlayAnimMontage` "/Game/Blueprints/Enemies/AM_GruntHit.AM_GruntHit" 1.0 "ROOT_WaistKnockBackHit" :!label _label_5))
    (:`Grunt_LeftUpLeg`
      (goto _label_5))
    (:`Grunt_RightUpLeg`
      (goto _label_5))
    (:`Grunt_Spine1`
      (goto _label_5))
    (:`Grunt_Spine2`
      (goto _label_5))))

(event `/Game/Blueprints/Enemies/AI/BPI_EnemyAI.JumpToDestination`
  (params (Destination :type "Vector Structure"))
  ;[1 1 1] Navigation Jump
  (bind _outlaunchvelocity (`GameplayStatics.SuggestProjectileVelocity_CustomArc` (`self.K2_GetActorLocation`) (`KismetMathLibrary.MakeVector` Destination_X Destination_Y (+ Destination_Z 150.0))))
  (`self.PlayAnimMontage` "/Game/Blueprints/Enemies/AM_GruntJump.AM_GruntJump" 1.0 "Grunt_JumpUp")
  (`self.LaunchCharacter` _outlaunchvelocity true true))

(event `self.OnLanded`
  (params (Hit :type "HitResult Structure (by ref)"))
  ;[1 1 1] Navigation Jump
  (`self.PlayAnimMontage` "/Game/Blueprints/Enemies/AM_GruntJump.AM_GruntJump" 1.0 "Grunt_JumpLand"))

(fn `GetIdealRange`
  (returns (AttackRadius :type "Float (double-precision)") (DefendRadius :type "Float (double-precision)"))
  (return 800.0 800.0))

(fn `UserConstructionScript`)