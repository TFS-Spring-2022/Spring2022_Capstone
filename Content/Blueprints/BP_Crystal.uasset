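; BP_Crystal is a damageable crystal that spawns a damage-over-time radius actor (BP_DOTRadiusCrystal) at its transform when hit.
; Each hit starts a cooldown matching the cloud's lifetime, during which further damage triggers nothing.
; A dynamic material instance shows the state, switching GlowColor to red during cooldown and restoring the cached base color afterward.
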(event `self.ReceiveBeginPlay`
  (bind _staticmesh (`self.StaticMesh`))
  (bind _returnvalue (`PrimitiveComponent.CreateDynamicMaterialInstance` _staticmesh 0 (`PrimitiveComponent.GetMaterial` _staticmesh 0) "None"))
  (bind _output_get (set `self.CrystalMaterial` _returnvalue))
  (bind _returnvalue_2 (`MaterialInstanceDynamic.K2_GetVectorParameterValue` _output_get "GlowColor"))
  (set `self.BaseColor` _returnvalue_2)
  (add `self.OnTakeAnyDamage` (delegate `OnTakeDamage`)))

(event `OnTakeDamage` :!signature `self.OnTakeAnyDamage`
  (params (DamagedActor :type "Actor Object Reference") (Damage :type "Float (single-precision)") (DamageType :type "DamageType Object Reference") (InstigatedBy :type "Controller Object Reference") (DamageCauser :type "Actor Object Reference"))
  (if (`self.bCanBeDamaged`)
    (`|SpawnActorFromClass` "/Game/Blueprints/BP_DOTRadiusCrystal.BP_DOTRadiusCrystal_C" (`self.GetTransform`) "Undefined" "OverrideRootScale" null 10.0 6.0 500.0 null)
    (`self.DeactivateTimer`)))

(event `DeactivateTimer`
  (set `self.bCanBeDamaged` false)
  (`self.ChangeMaterial`)
  (`KismetSystemLibrary.Delay` 6.0)
  (set `self.bCanBeDamaged` true)
  (`self.ChangeMaterial`))

(event `ChangeMaterial`
  (if (`self.bCanBeDamaged`)
    (`MaterialInstanceDynamic.SetVectorParameterValue` (`self.CrystalMaterial`) "GlowColor" (`self.BaseColor`))
    (else
      (`MaterialInstanceDynamic.SetVectorParameterValue` (`self.CrystalMaterial`) "GlowColor" (`KismetMathLibrary.MakeColor` 1.0 0.0 0.0 0.0)))))

(fn `UserConstructionScript`)