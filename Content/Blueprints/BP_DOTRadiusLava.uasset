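; BP_DOTRadiusLava is a lava damage-over-time area that hurts an overlapping actor that has a HealthComponent.
; Sphere begin overlap stores that actor in a single reference and starts a looping two-second DealDamage timer.
; Each tick applies DamagePerSecond through ApplyDamage and prints the result.
; End overlap only compares the actor, so the timer and reference are never cleared and damage continues after exit.
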(event `self.SphereCollision.OnComponentBeginOverlap`
  (params (OverlappedComponent :type "PrimitiveComponent Object Reference") (OtherActor :type "Actor Object Reference") (OtherComp :type "PrimitiveComponent Object Reference") (OtherBodyIndex :type Integer) (bFromSweep :type Boolean) (SweepResult :type "HitResult Structure (by ref)"))
  (`/Engine/EditorBlueprintResources/StandardMacros.IsValid` (`self.GetComponentByClass` OtherActor "/Script/Spring2022_Capstone.HealthComponent")
    (:`Is Valid`
      (set `self.OtherCharRef` OtherActor)
      (`KismetSystemLibrary.K2_SetTimer` null "DealDamage" 2.0 true))))

(event `DealDamage`
  (bind _othercharref (`self.OtherCharRef`)
    (:`then`
      (bind _returnvalue (`GameplayStatics.ApplyDamage` _othercharref (`self.DamagePerSecond`)))
      (`KismetSystemLibrary.PrintString` (`KismetStringLibrary.Concat_StrStr` "Dealing damage of: " (`KismetStringLibrary.Conv_DoubleToString` _returnvalue))))
    (:`else`)))

(event `self.SphereCollision.OnComponentEndOverlap`
  (params (OverlappedComponent :type "PrimitiveComponent Object Reference") (OtherActor :type "Actor Object Reference") (OtherComp :type "PrimitiveComponent Object Reference") (OtherBodyIndex :type Integer))
  (if (== OtherActor (`self.OtherCharRef`))
    _))

(fn `UserConstructionScript`)