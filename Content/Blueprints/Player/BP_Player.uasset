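; Player Blueprint whose event graph holds debug key bindings for testing upgrades, health and wave spawning.
; Number and numpad keys call UpgradeSystemComponent to boost health, speed, double jump and grapple cooldown, or upgrade the active weapon's damage and charge.
; Other keys heal or damage the player, toggle the upgrade menu and trigger a debug wave spawn from the Game Mode's Wave Manager.
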(event `Key|One`
  (params (Key :type "Key Structure"))
  ;[1 1 1] Upgrade System Testing
  (:`Pressed`
    (`UpgradeSystemComponent.IncreaseMaxHealthByAmount` (`self.UpgradeSystemComponent`) 10.0)))

(event `Key|Two`
  (params (Key :type "Key Structure"))
  ;[1 1 1] Upgrade System Testing
  (:`Pressed`
    (`UpgradeSystemComponent.IncreaseMaxHealthByPercentage` (`self.UpgradeSystemComponent`) 50.0)))

(event `Key|Three`
  (params (Key :type "Key Structure"))
  ;[1 1 1] Upgrade System Testing
  (:`Pressed`
    (`UpgradeSystemComponent.IncreaseMovementSpeedByAmount` (`self.UpgradeSystemComponent`) 5)))

(event `Key|NumPadOne`
  (params (Key :type "Key Structure"))
  ;[1 1 1] Upgrade System Testing
  (:`Pressed`
    (bind _returnvalue (`self.GetActiveWeapon`))
    (`UpgradeSystemComponent.IncreaseMaxChargeAmount` (`self.UpgradeSystemComponent`) _returnvalue 10.0)))

(event `Key|Four`
  (params (Key :type "Key Structure"))
  ;[1 1 1] Upgrade System Testing
  (:`Pressed`
    (bind _returnvalue (`self.GetActiveWeapon`))
    (`UpgradeSystemComponent.IncreaseWeaponDamageByAmount` (`self.UpgradeSystemComponent`) _returnvalue 50.0)))

(event `Key|Five`
  (params (Key :type "Key Structure"))
  ;[1 1 1] Upgrade System Testing
  (:`Pressed`
    (`UpgradeSystemComponent.UnlockDoubleJump` (`self.UpgradeSystemComponent`))))

(event `Key|Six`
  (params (Key :type "Key Structure"))
  ;[1 1 1] Upgrade System Testing
  (:`Pressed`
    (`UpgradeSystemComponent.DecreaseGrappleCooldownBySeconds` (`self.UpgradeSystemComponent`) 1.0)))

(event `Key|Seven`
  (params (Key :type "Key Structure"))
  ;[1 1 1] Upgrade System Testing
  (:`Pressed`
    (bind _returnvalue (`self.GetActiveWeapon`))
    (`UpgradeSystemComponent.IncreaseChargeCooldownRate` (`self.UpgradeSystemComponent`) _returnvalue 1.0)))

(event `Key|C`
  (params (Key :type "Key Structure"))
  ;[1 1 1] Heal & Damage
  (:`Pressed`
    (`self.Heal` 5)))

(event `Key|X`
  (params (Key :type "Key Structure"))
  ;[1 1 1] Heal & Damage
  (:`Pressed`
    (`self.DamageActor` self 10.0)))

(event `Key|P` :paused true
  (params (Key :type "Key Structure"))
  (bind _upgradesystemcomponent (`self.UpgradeSystemComponent`))
  ;[1 1 1] Open Upgrade Menu
  (:`Pressed`
    (if (`UpgradeSystemComponent.bIsMenuOpen` _upgradesystemcomponent)
      (`UpgradeSystemComponent.CloseUpgradeMenu` _upgradesystemcomponent)
      (else
        (`UpgradeSystemComponent.OpenUpgradeMenu` _upgradesystemcomponent)))))

(event `Key|J`
  (params (Key :type "Key Structure"))
  ;[1 1 1] Spawn a wave from Game Mode's Wave Manager
  (:`Pressed`
    (`self.DEBUG_SpawnWave`)))

(fn `UserConstructionScript`)