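; Test player character Blueprint with camera-relative look and movement input, plus a hold-to-grapple hook on Left Shift.
; Pressing line-traces from the camera and, on a hit, switches movement to Flying and shows the cable.
; Tick pins the cable end to the impact point and applies constant force toward it.
; Every release restores Falling, hides the cable and starts a cooldown, even without a hit.
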(event `InputAxis|Horizontal Look`
  (params (AxisValue :type "Float (single-precision)"))
  ;[1 1 1] Player Look
  (`self.AddControllerYawInput` AxisValue))

(event `InputAxis|Vertical Look`
  (params (AxisValue :type "Float (single-precision)"))
  ;[1 1 1] Player Look
  (`self.AddControllerPitchInput` AxisValue))

(event `InputAxis|Movement Forward/Backward`
  (params (AxisValue :type "Float (single-precision)"))
  ;[1 1 1] Player Movement
  (`self.AddMovementInput` (`SceneComponent.GetForwardVector` (`self.Camera`)) AxisValue))

(event `InputAxis|Movement Strafe`
  (params (AxisValue :type "Float (single-precision)"))
  ;[1 1 1] Player Movement
  (`self.AddMovementInput` (`SceneComponent.GetRightVector` (`self.Camera`)) AxisValue))

(event `Key|LeftShift`
  (params (Key :type "Key Structure"))
  (bind _camera (`self.Camera`))
  (bind _returnvalue (`SceneComponent.K2_GetComponentLocation` _camera))
  ;[1 1 1] Grappling Mechanic
  (:`Pressed`
    (if (`self.canGrapple`)
      (bind (_outhit _returnvalue_2) (`KismetSystemLibrary.LineTraceSingle` _returnvalue (+ _returnvalue (* (`KismetMathLibrary.GetForwardVector` (`SceneComponent.K2_GetComponentRotation` _camera)) 3000.0)) "TraceTypeQuery1"))
      (if _returnvalue_2
        (set `self.hookImpactPoint` (`.ImpactPoint` (`GameplayStatics.BreakHitResult` _outhit)))
        (set `self.isGrappling` true)
        (`CharacterMovementComponent.SetMovementMode` (`self.CharacterMovement`) "MOVE_Flying" 0)
        (`SceneComponent.SetVisibility` (`self.Cable`) true false))))
  (:`Released`
    (set `self.isGrappling` false)
    (`CharacterMovementComponent.SetMovementMode` (`self.CharacterMovement`) "MOVE_Falling" 0)
    (`SceneComponent.SetVisibility` (`self.Cable`) false false)
    (set `self.canGrapple` false)
    (`KismetSystemLibrary.Delay` (`self.grappleCooldown`))
    (set `self.canGrapple` true)))

(event `self.ReceiveTick`
  (params (DeltaSeconds :type "Float (single-precision)"))
  ;[1 1 1] Grappling Mechanic
  (if (`self.isGrappling`)
    (set `CableComponent.EndLocation` (`KismetMathLibrary.InverseTransformLocation` (`self.GetTransform`) (`self.hookImpactPoint`)) (`self.Cable`))
    (`CharacterMovementComponent.AddForce` (`self.CharacterMovement`) (* (`KismetMathLibrary.Normal` (`KismetMathLibrary.GetDirectionUnitVector` (`self.K2_GetActorLocation`) (`self.hookImpactPoint`))) 300000.0))))

(fn `UserConstructionScript`)